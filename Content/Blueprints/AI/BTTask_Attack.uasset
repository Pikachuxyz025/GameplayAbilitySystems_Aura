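; Behavior tree task that makes an enemy pawn attack the target stored in its blackboard.
; On AI execute, it checks that the pawn implements EnemyInterface and the AttackTarget key holds a valid actor, then passes that actor to SetCombatTarget.
; It activates Gameplay Ability System abilities matching AttackTag and finishes successfully immediately, without waiting on the ability, or fails if either check fails.
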(event `self.ReceiveExecuteAI`
  (params (OwnerController :type "AIController Object Reference") (ControlledPawn :type "Pawn Object Reference"))
  (bind _returnvalue (`BTFunctionLibrary.GetBlackboardValueAsActor` (`self.AttackTarget`)))
  (bind _asenemy_interface (cast `EnemyInterface` ControlledPawn)
    (:`then`
      (`/Engine/EditorBlueprintResources/StandardMacros.IsValid` _returnvalue
        (:`Is Valid`
          (`EnemyInterface.SetCombatTarget` _asenemy_interface _returnvalue)
          (`AbilitySystemComponent.TryActivateAbilitiesByTag` (`AbilitySystemBlueprintLibrary.GetAbilitySystemComponent` ControlledPawn) (`BlueprintGameplayTagLibrary.MakeGameplayTagContainerFromTag` (`self.AttackTag`)) true)
          (`self.FinishExecute` true))
        (:`Is Not Valid`
          (`self.FinishExecute` false :!label _label))))
    (:`CastFailed`
      (goto _label))))