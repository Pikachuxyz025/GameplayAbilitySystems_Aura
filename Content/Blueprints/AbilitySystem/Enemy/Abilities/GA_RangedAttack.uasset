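; Enemy ranged attack gameplay ability that fires a projectile at the avatar's current combat target.
; On activation it turns the avatar toward the target and plays a random tagged montage from the avatar's attack montages.
; The montage's gameplay event triggers SpawnProjectile from the tagged socket at the target's then-current location, with an optional pitch override.
; The ability ends when the montage completes, is interrupted or is cancelled.
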(event `self.K2_ActivateAbility`
  (bind _returnvalue (`self.GetAvatarActorFromActorInfo`))
  (bind (_taggedvariable_montage _taggedvariable_montagetag _taggedvariable_sockettag) (break `TaggedMontage` (`self.TaggedVariable`)))
  (bind (_taggedvariable_montage_2 _taggedvariable_montagetag_2) (break `TaggedMontage` (`self.TaggedVariable`)))
  (bind _ascombat_interface (cast `CombatInterface` _returnvalue))
  (bind _returnvalue_2 (message `EnemyInterface.GetCombatTarget` _returnvalue))
  (`CombatInterface.UpdateFacingTarget` _ascombat_interface (`Actor.K2_GetActorLocation` _returnvalue_2))
  (bind _returnvalue_3 (message `CombatInterface.GetAttackMontages` _returnvalue))
  (bind _output_get (set `self.TaggedVariable` (`self.GetRandomTaggedMontageFromArray` _returnvalue_3)))
  (`AbilityTask_PlayMontageAndWait.CreatePlayMontageAndWaitProxy` "None" (`.Montage` (break `TaggedMontage` _output_get)) 1.0 "None" false
    (:`then`
      (`AbilityTask_WaitGameplayEvent.WaitGameplayEvent` _taggedvariable_montagetag_2 null true
        (:`EventReceived`
          (`KismetSystemLibrary.PrintString` "Shots Fired")
          (bind _returnvalue_4 (message `EnemyInterface.GetCombatTarget` (`self.GetAvatarActorFromActorInfo`)))
          (`self.SpawnProjectile` (`Actor.K2_GetActorLocation` _returnvalue_4) _taggedvariable_sockettag (`self.Should Override Pitch`) (`self.Pitch Override`)))))
    (:`OnCompleted`
      (`self.K2_EndAbility` :!label _label))
    (:`OnInterrupted`
      (goto _label))
    (:`OnCancelled`
      (goto _label))))