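; GA_ListenForEvents is a passive startup ability that turns attribute gameplay events into effects on its owner.
; On activation it waits for any event under the Attributes tag, then MakeSpecHandle looks up that tag's effect class in the EffectsClasses map.
; When found, it sets the event magnitude as SetByCaller and applies the spec to self.
; An unconnected alternative uses one shared effect, zeroing non-matching tags.
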(event `self.K2_ActivateAbility`
  (bind (_asynctaskproxy _payload) (`AbilityTask_WaitGameplayEvent.WaitGameplayEvent` (struct :`TagName` "Attributes") null false false)
    (:`EventReceived`
      (bind (_eventtag _instigator _target _optionalobject _optionalobject2 _contexthandle _instigatortags _targettags _eventmagnitude) (break `GameplayEventData` _payload))
      (bind _output_get (set `self.Event Tag` _eventtag))
      (set `self.Event Magnitude` _eventmagnitude)
      (bind (_bsuccess _outspec) (`self.MakeSpecHandle` _output_get))
      (if _bsuccess
        (bind _returnvalue (`AbilitySystemBlueprintLibrary.AssignTagSetByCallerMagnitude` _outspec (`self.Event Tag`) (`self.Event Magnitude`)))
        (`AbilitySystemComponent.BP_ApplyGameplayEffectSpecToSelf` (`self.GetAbilitySystemComponentFromActorInfo`) _returnvalue)))))

(fn `MakeSpecHandle`
  (params (AttributeTag :type "GameplayTag Structure (by ref)"))
  (returns (bSuccess :type Boolean) (OutSpec :type "GameplayEffectSpecHandle Structure"))
  (bind _returnvalue (`self.GetAbilitySystemComponentFromActorInfo`))
  (bind (_value _returnvalue_2) (`BlueprintMapLibrary.Map_Find` (`self.EffectsClasses`) AttributeTag))
  (if _returnvalue_2
    _
    (else
      _))
  (return _returnvalue_2 (`AbilitySystemComponent.MakeOutgoingSpec` _returnvalue _value 1.0 (`AbilitySystemComponent.MakeEffectContext` _returnvalue))))