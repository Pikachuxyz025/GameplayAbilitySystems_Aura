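; Gameplay ability for the Firebolt spell, which launches a projectile toward the location under the mouse.
; On activation it commits without branching on the result, gets target data under the mouse and turns the avatar toward it through CombatInterface.
; It plays the cast montage, spawns the projectile from the weapon socket when the montage's gameplay event arrives, and ends on montage completion.
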(event `self.K2_ActivateAbility`
  (bind _returnvalue (`self.K2_CommitAbility`))
  (`KismetSystemLibrary.PrintString` (`KismetStringLibrary.Conv_BoolToString` _returnvalue))
  (bind (_asynctaskproxy _datahandle) (`AT_TargetDataUnderMouse.CreateTargetDataUnderMouse`)
    (:`ValidData`
      (set `self.ProjectileTargetLocation` (`.Location` (`GameplayStatics.BreakHitResult` (`AbilitySystemBlueprintLibrary.GetHitResultFromTargetData` _datahandle))))
      (bind _ascombat_interface (cast `CombatInterface` (`self.GetAvatarActorFromActorInfo`)))
      (`CombatInterface.UpdateFacingTarget` _ascombat_interface (`self.ProjectileTargetLocation`))
      (`AbilityTask_PlayMontageAndWait.CreatePlayMontageAndWaitProxy` "None" "/Game/Assets/Characters/Aura/Animations/Abilities/AM_Cast_Firebolt.AM_Cast_Firebolt" 1.0 "None" false
        (:`then`
          (`AbilityTask_WaitGameplayEvent.WaitGameplayEvent` (struct :`TagName` "Event.Montage.FireBolt") null
            (:`EventReceived`
              (`KismetSystemLibrary.PrintString` "Firebolt Event Recieved" true true (struct :`R` 1.0 :`G` 0.7573 :`B` 0.339465 :`A` 1.0))
              (`self.SpawnProjectile` (`self.ProjectileTargetLocation`) (`BlueprintGameplayTagLibrary.MakeLiteralGameplayTag` (struct :`TagName` "CombatSocket.Weapon"))))))
        (:`OnCompleted`
          (`self.K2_EndAbility`))))))